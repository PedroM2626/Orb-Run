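; BP_OrangeOrb is an orange orb pickup that Carlinhos collects by overlapping it.
; Collection increases the character's orange orb count, destroys the orb and asks BP_OrbsSpawner to spawn another.
; An uncollected orb destroys itself after a three-second Delay driven from Tick and triggers the same respawn call.
; A timeline started at BeginPlay animates the sphere's relative Z location.
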(event `self.ReceiveActorBeginOverlap`
  (params (OtherActor :type "Actor Object Reference"))
  (bind _ascarlinhos (cast `/Game/Blueprints/RetargetedCharacters/Carlinhos` OtherActor))
  (`/Game/Blueprints/RetargetedCharacters/Carlinhos.IncreaseOrbO` _ascarlinhos)
  (`self.K2_DestroyActor`)
  (bind _returnvalue (`GameplayStatics.GetActorOfClass` "/Game/Orbs/BP_OrbsSpawner.BP_OrbsSpawner_C" :!label _label))
  (`/Game/Orbs/BP_OrbsSpawner.SpawnOrbO` _returnvalue))

(event `self.ReceiveTick`
  (params (DeltaSeconds :type "Float (single-precision)"))
  (`KismetSystemLibrary.Delay` 3.0)
  (`self.K2_DestroyActor`)
  (goto _label))

(event `self.ReceiveBeginPlay`
  (bind (_direction _nova_faixa_0) (`Timeline|Linha do tempo`)
    (:`Update`
      (`SceneComponent.K2_SetRelativeLocation` (`self.Sphere`) (`KismetMathLibrary.MakeVector` 0.0 0.0 _nova_faixa_0) false false))))

(fn `UserConstructionScript`)
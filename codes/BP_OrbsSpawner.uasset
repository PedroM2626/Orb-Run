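; Spawner actor that places normal, golden and orange orbs at random points from its SpawnLocations array.
; BeginPlay spawns a normal orb, while SpawnOrbG and SpawnOrbO have no caller in this Blueprint.
; Each function compares its pick with the other orbs' stored transforms and rerolls once on a match, without rechecking.
; Normal and orange also avoid their own previous spot, but golden's equivalent check is unconnected.
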(event `self.ReceiveBeginPlay`
  (`self.SpawnOrbN`))

(fn `SpawnOrbG`
  (bind _output_get (set `self.OrbGpostition` (`self.GetTransform` (`KismetArrayLibrary.Array_Random` (`self.SpawnLocations`)))))
  (if (or (or (`KismetMathLibrary.NearlyEqual_TransformTransform` _output_get (`self.OrbOposition`) 0.0 0.0 1e-05) (`KismetMathLibrary.NearlyEqual_TransformTransform` _output_get (`self.OrbNposition`) 0.0 0.0 1e-05)) false)
    (bind _output_get_2 (set `self.OrbGpostition` (`self.GetTransform` (`KismetArrayLibrary.Array_Random` (`self.SpawnLocations`)))))
    (bind _output_get_3 (set `self.ApositionG` _output_get_2))
    (`|SpawnActorFromClass` "/Game/Orbs/BP_GoldenOrb.BP_GoldenOrb_C" _output_get_3 "AdjustIfPossibleButDontSpawnIfColliding" "MultiplyWithRoot" null null)
    (else
      (`|SpawnActorFromClass` "/Game/Orbs/BP_GoldenOrb.BP_GoldenOrb_C" _output_get "AdjustIfPossibleButDontSpawnIfColliding" "MultiplyWithRoot" null null))))

(fn `SpawnOrbN`
  (bind _output_get (set `self.OrbNposition` (`self.GetTransform` (`KismetArrayLibrary.Array_Random` (`self.SpawnLocations`)))))
  (if (or (or (`KismetMathLibrary.NearlyEqual_TransformTransform` _output_get (`self.OrbOposition`) 0.0 0.0 1e-05) (`KismetMathLibrary.NearlyEqual_TransformTransform` _output_get (`self.OrbGpostition`) 0.0 0.0 1e-05)) (`KismetMathLibrary.NearlyEqual_TransformTransform` (`self.OrbNposition`) (`self.ApositionN`) 0.0 0.0 1e-05))
    (bind _output_get_2 (set `self.OrbNposition` (`self.GetTransform` (`KismetArrayLibrary.Array_Random` (`self.SpawnLocations`)))))
    (bind _output_get_3 (set `self.ApositionN` _output_get_2))
    (`|SpawnActorFromClass` "/Game/Orbs/BP_Orb.BP_Orb_C" _output_get_3 "AdjustIfPossibleButDontSpawnIfColliding" "MultiplyWithRoot" null null)
    (else
      (bind _output_get_4 (set `self.ApositionN` _output_get))
      (`|SpawnActorFromClass` "/Game/Orbs/BP_Orb.BP_Orb_C" _output_get_4 "AdjustIfPossibleButDontSpawnIfColliding" "MultiplyWithRoot" null null))))

(fn `SpawnOrbO`
  (bind _output_get (set `self.OrbOposition` (`self.GetTransform` (`KismetArrayLibrary.Array_Random` (`self.SpawnLocations`)))))
  (if (or (or (`KismetMathLibrary.NearlyEqual_TransformTransform` _output_get (`self.OrbGpostition`) 0.0 0.0 1e-05) (`KismetMathLibrary.NearlyEqual_TransformTransform` _output_get (`self.OrbNposition`) 0.0 0.0 1e-05)) (`KismetMathLibrary.NearlyEqual_TransformTransform` (`self.ApositionO`) (`self.OrbOposition`) 0.0 0.0 1e-05))
    (bind _output_get_2 (set `self.OrbOposition` (`self.GetTransform` (`KismetArrayLibrary.Array_Random` (`self.SpawnLocations`)))))
    (bind _output_get_3 (set `self.ApositionO` _output_get_2))
    (`|SpawnActorFromClass` "/Game/Orbs/BP_OrangeOrb.BP_OrangeOrb_C" _output_get_3 "AdjustIfPossibleButDontSpawnIfColliding" "MultiplyWithRoot" null null)
    (else
      (bind _output_get_4 (set `self.ApositionO` _output_get))
      (`|SpawnActorFromClass` "/Game/Orbs/BP_OrangeOrb.BP_OrangeOrb_C" _output_get_4 "AdjustIfPossibleButDontSpawnIfColliding" "MultiplyWithRoot" null null))))

(fn `UserConstructionScript`)